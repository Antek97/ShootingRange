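; Shotgun projectile actor that destroys itself on hit and prints its display name.
; On begin play it stores the static mesh's world rotation in StartPosition.
; A Rotate flag toggles on tick, and every other tick sets the mesh's relative yaw to one degree past that stored yaw, with zero pitch and roll.
; The stored rotation never updates, so the yaw offset does not accumulate.
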(event EventTick
  (params (DeltaSeconds :type Float%20%28single-precision%29))
  (if (Variables|Default|GetbRotate)
    (Transformation|SetRelativeRotation (Variables|Default|GetStaticMesh) (Math|Rotator|MakeRotator 0.0 0.0 (+ (.yaw (Variables|Default|GetStartPosition)) 1.0)) false false)
    (Variables|Default|SetbRotate false)
    (else
      (Variables|Default|SetbRotate true))))

(event Collision|EventHit
  (params (MyComp :type Primitive%20Component%20Object%20Reference) (Other :type Actor%20Object%20Reference) (OtherComp :type Primitive%20Component%20Object%20Reference) (bSelfMoved :type Boolean) (HitLocation :type Vector :default "0, 0, 0") (HitNormal :type Vector :default "0, 0, 0") (NormalImpulse :type Vector :default "0, 0, 0") (Hit :type Hit%20Result%20Structure%20%28by%20ref%29))
  (Actor|DestroyActor)
  (Development|PrintString (Utilities|GetDisplayName self)))

(event EventBeginPlay
  (Variables|Default|SetStartPosition (Transformation|GetWorldRotation (Variables|Default|GetStaticMesh))))

(fn ConstructionScript)