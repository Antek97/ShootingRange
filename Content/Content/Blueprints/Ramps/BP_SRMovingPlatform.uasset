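; Shooting range platform that slides between its start position and a lifted position when a ShootingRangeCharacter begins overlapping it.
; BeginPlay caches the actor's location and converts MaximumLift from an offset into an absolute target.
; Each overlap compares actor location to the start to pick the destination, then MoveComponentTo moves the mesh there, passing these world positions as relative targets.
; End overlap checks the class but does nothing.
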(event EventBeginPlay
  (bind _self self)
  (bind _returnvalue (Transformation|GetActorLocation _self))
  (Variables|Default|SetStartPositionLift _returnvalue)
  (Variables|Components|SetMaximumLift%20 (+ _returnvalue (Variables|Components|GetMaximumLift%20))))

(event Collision|EventActorBeginOverlap
  (params (OtherActor :type Actor%20Object%20Reference))
  (if (Utilities|ClassIsChildOf (Utilities|GetClass OtherActor) "/Script/ShootingRange.ShootingRangeCharacter")
    (Components|MoveComponentTo (Variables|Default|GetPlatformStaticMesh) (Math|Vector|SelectVector (Variables|Default|GetStartPositionLift) (Variables|Components|GetMaximumLift%20) (Class|KismetMathLibrary|NotEqualExactlyVectorVector (Transformation|GetActorLocation self) (Variables|Default|GetStartPositionLift))) "0, 0, 0" false false 1.0 false)))

(event Collision|EventActorEndOverlap
  (params (OtherActor :type Actor%20Object%20Reference))
  (if (Utilities|ClassIsChildOf (Utilities|GetClass OtherActor) "/Script/ShootingRange.ShootingRangeCharacter")
    _))

(fn ConstructionScript)